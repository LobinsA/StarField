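; Navigational guide actor that shows waypoint markers along the navmesh route from the player to itself.
; A looping one-second timer finds the path synchronously, adds its points to a spline and spawns three static mesh components at fixed distances along it.
; After a one-second delay it clears the spline points and destroys the markers, so the trail is regularly rebuilt from the player's current location.
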(event `self.ReceiveBeginPlay`
  (`KismetSystemLibrary.K2_SetTimerDelegate` (delegate `BuildNav`) 1.0 true))

(event `BuildNav`
  (bind _path_points (`self.FindPath`))
  (`self.BuildSpline` _path_points)
  (`self.BuildPath`)
  (`KismetSystemLibrary.Delay` 1.0)
  (`self.ClearSpline`))

(fn `BuildPath`
  (for _index (range 3)
    (bind _returnvalue (`AddComponent|NODE_AddStaticMeshComponent-0`))
    (`SceneComponent.K2_SetWorldLocation` _returnvalue (`SplineComponent.GetLocationAtDistanceAlongSpline` (`self.Spline`) (* (+ _index 1) 500) "World") false false)
    (`KismetArrayLibrary.Array_Add` (`self.WaypointList`) _returnvalue)))

(fn `BuildSpline`
  (params (PathPoints :type "Array of Vector Structure"))
  (for _array_element PathPoints
    (`SplineComponent.AddSplinePoint` (`self.Spline`) _array_element "World" true)))

(fn `ClearSpline`
  (`SplineComponent.ClearSplinePoints` (`self.Spline`) true)
  (for _array_element (`self.WaypointList`)
    (`ActorComponent.K2_DestroyComponent` _array_element))
  (`KismetArrayLibrary.Array_Clear` (`self.WaypointList`)))

(fn `FindPath`
  (returns (`Path Points` :type "Array of Vector Structure"))
  (bind _returnvalue (`NavigationSystemV1.FindPathToActorSynchronously` (`self.K2_GetActorLocation` (`GameplayStatics.GetPlayerCharacter` 0)) self 50.0 null null))
  (`/Engine/EditorBlueprintResources/StandardMacros.IsValid` _returnvalue
    (:`Is Valid`
      (return (`NavigationPath.PathPoints` _returnvalue)))))

(fn `UserConstructionScript`)