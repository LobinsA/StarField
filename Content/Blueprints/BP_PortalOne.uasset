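; BP_PortalOne is an actor that opens a portal in front of the player when something overlaps it.
; On overlap, it spawns the P_PortalEffect particle and a scaled-up BP_StreamingLevelOne actor at a fixed distance along the player camera's forward vector.
; The spawned actor has a limited life span, and the stored Emitter reference blocks respawning while valid, printing a debug message instead.
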(event `self.ReceiveBeginPlay`)

(event `self.ReceiveActorBeginOverlap`
  (params (OtherActor :type "Actor Object Reference"))
  (bind _returnvalue (`GameplayStatics.GetPlayerCameraManager` 0))
  (bind _returnvalue_2 (+ (* (`self.GetActorForwardVector` _returnvalue) 1500) (`self.K2_GetActorLocation` _returnvalue)))
  (if (`KismetSystemLibrary.IsValid` (`self.Emitter`))
    (`KismetSystemLibrary.PrintString` "Emitter Exists")
    (else
      (bind _returnvalue_3 (`GameplayStatics.SpawnEmitterAtLocation` "/Game/Effects/P_PortalEffect.P_PortalEffect" _returnvalue_2))
      (set `self.Emitter` _returnvalue_3)
      (bind _returnvalue_4 (`|SpawnActorFromClass` "/Game/Blueprints/BP_StreamingLevelOne.BP_StreamingLevelOne_C" (`KismetMathLibrary.MakeTransform` _returnvalue_2 (struct) (5.0 5.0 5.0)) "AdjustIfPossibleButAlwaysSpawn" "OverrideRootScale" null null))
      (`self.SetLifeSpan` _returnvalue_4 10.0))))

(fn `UserConstructionScript`)